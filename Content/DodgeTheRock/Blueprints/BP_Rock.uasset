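; BP_Rock is a moving rock hazard for DodgeTheRock that turns toward the player pawn on spawn and flies straight along its forward vector.
; Tick moves it with a swept world offset, so collisions fire a hit event bound at BeginPlay.
; Hitting an actor tagged Player deals damage and destroys the rock; any other hit bounces it by reflecting its direction off the surface normal, flattened to 2D.
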(event Custom|OnActorHit_Event
  (params (SelfActor :type Actor%20Object%20Reference) (OtherActor :type Actor%20Object%20Reference) (NormalImpulse :type Vector) (Hit :type Hit%20Result%20Structure%20%28by%20ref%29))
  (if (Actor|ActorHasTag OtherActor "Player")
    (Game|Damage|ApplyDamage OtherActor (Variables|Default|GetBase%20Damage) 0 self)
    (Actor|DestroyActor)
    (else
      (Transformation|SetActorRotation (Math|Rotator|MakeRotfromX (Class|KismetMathLibrary|VectorNormal2D (Math|Vector|GetReflectionVector (Transformation|GetActorForwardVector) (.Normal (Collision|BreakHitResult Hit))) 0.0001))))))

(event EventTick
  (params (DeltaSeconds :type Float%20%28single-precision%29))
  (Transformation|AddActorWorldOffset (* (* DeltaSeconds (Variables|Gameplay|GetSpeed)) (Transformation|GetActorForwardVector)) true))

(event EventBeginPlay
  (Utilities|FlowControl|Sequence
    (:then_0
      (Utilities|TurntoPlayer) ; rotating rock to face pawn
    )
    (:then_1
      (Collision|BindEventtoOnActorHit (EventDispatchers|CreateEvent :!event Custom|OnActorHit_Event)))))

(fn ConstructionScript)