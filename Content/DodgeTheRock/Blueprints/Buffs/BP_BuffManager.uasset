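; Buff manager for DodgeTheRock that keeps a single random buff in the level, respawning it after pickup.
; On BeginPlay, only if the spawner array is already non-empty, it refills it with all BP_BuffSpawner actors and spawns after a short delay.
; Each spawn picks a random class and spawner transform, passing itself to the buff.
; BuffPicked destroys the buff, clears the reference and schedules the next spawn.
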(event Custom|SpawnRandomBuff
  (Variables|Default|GetCurrentBuffRef
    (:then)
    (:else
      (bind _returnvalue (Game|SpawnActorfromClass (.OutItem (Utilities|Array|Random (Variables|Default|GetBuffClasses))) (Transformation|GetActorTransform (.OutItem (Utilities|Array|Random (Variables|Default|GetBuffSpawners)))) "Undefined" "MultiplyWithRoot" 0 self 0))
      (Variables|Default|SetCurrentBuffRef _returnvalue))))

(event Custom|BuffPicked
  (params (BuffPicked :type BP%20Buff%20Object%20Reference))
  (Actor|DestroyActor BuffPicked)
  (Variables|Default|SetCurrentBuffRef 0)
  (Variables|Default|GetCurrentBuffRef
    (:then)
    (:else
      (Utilities|FlowControl|Delay 3.0)
      (CallFunction|SpawnRandomBuff))))

(event EventBeginPlay
  (if (Utilities|Array|IsNotEmpty (Variables|Default|GetBuffSpawners))
    (bind _outactors (Actor|GetAllActorsOfClass "/Game/DodgeTheRock/Blueprints/Buffs/BP_BuffSpawner.BP_BuffSpawner_C"))
    (Variables|Default|SetBuffSpawners _outactors)
    (Utilities|FlowControl|Delay 1.0)
    (CallFunction|SpawnRandomBuff)))

(fn ConstructionScript)