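; BP_RockSpawner spawns BP_Rock actors at random positions for the dodge-the-rock game.
; On BeginPlay it sets the base rock damage from the game instance's difficulty, with harder settings dealing more.
; SpawnRockInVolume takes random X and Y inside the Box bounds, keeps Z at the spawner's height and passes that damage to the rock.
; The file contains no timer or call that triggers the spawn event.
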(event Custom|SpawnRockInVolume
  (bind _box (Variables|Default|GetBox))
  (bind _returnvalue (Transformation|GetWorldLocation _box))
  (bind _returnvalue_2 (Components|Box|GetScaledBoxExtent _box))
  (bind _returnvalue_3 (Math|Random|RandomPointinBoundingBox _returnvalue _returnvalue_2))
  (bind (_x _y) (Math|Vector|BreakVector _returnvalue_3))
  (Game|SpawnActorfromClass "/Game/DodgeTheRock/Blueprints/BP_Rock.BP_Rock_C" (Math|Transform|MakeTransform (Math|Vector|MakeVector _x _y (.Z (Math|Vector|BreakVector (Transformation|GetActorLocation))))) "AdjustIfPossibleButAlwaysSpawn" "MultiplyWithRoot" 0 (Variables|Default|GetBaseRockDamage) 0))

(event EventBeginPlay
  (bind _asbp_dodge_game_instance (Utilities|Casting|CastToBP_DodgeGameInstance (Game|GetGameInstance)))
  (Variables|Default|SetBaseRockDamage (Utilities|Select :Index (Default|GetDificulty _asbp_dodge_game_instance) :NewEnumerator0 25.0 :NewEnumerator1 5e+01 :NewEnumerator2 1e+02)))

(fn ConstructionScript)