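; Game mode for DodgeTheRock that drives timed rock spawning and relays game end and restart to the game state.
; It caches the BP_DodgeGameState reference on BeginPlay for reuse by its events.
; Process calls SpawnRock whenever the supplied time is a multiple of five, then updates the game state's rock count.
; SpawnRock is an empty event here, while EndGame and RestartGame forward to the game state.
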(event Custom|Process
  (params (CurrentTime :type Integer))
  ;[0.15 0.15 0.15 0.5] Rock spawning each 5 sec
  (if (== (Math|Integer|%(Integer) CurrentTime 5) 0)
    (CallFunction|SpawnRock)
    (bind _dodgegamestate (Variables|Default|GetDodgeGameState)
      (:then
        (Default|SetRockCount _dodgegamestate (Math|Float|Truncate (stale _result))))
      (:else))))

(event Custom|SpawnRock)

(event Custom|EndGame
  (bind _dodgegamestate (Variables|Default|GetDodgeGameState)
    (:then
      (Default|EndGame _dodgegamestate))
    (:else)))

(event Custom|RestartGame
  (bind _dodgegamestate (Variables|Default|GetDodgeGameState)
    (:then
      (Default|RestartGame _dodgegamestate))
    (:else)))

(event EventBeginPlay
  ;[0.15 0.15 0.15 0.5] Casting GameState to a variable to reuse(Process, EndGame, RestartGame)
  (bind _asbp_dodge_game_state (Utilities|Casting|CastToBP_DodgeGameState (Game|GetGameState)))
  (Variables|Default|SetDodgeGameState _asbp_dodge_game_state))

(fn ConstructionScript)