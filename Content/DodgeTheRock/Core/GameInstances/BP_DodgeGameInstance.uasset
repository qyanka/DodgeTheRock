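; Game instance Blueprint for Dodge The Rock that holds the game difficulty and the highest score.
; Simple getter and setter functions expose both values.
; The high score setter overwrites the stored value only when the new score is greater, while difficulty is set directly.
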(fn SetDificulty
  (params (Dificulty :type E_GameDificulty%20Enum :default "NewEnumerator0"))
  (Variables|Default|SetGameDificulty Dificulty))

(fn GetDificulty
  (return (Variables|Default|GetGameDificulty)))

(fn SetHighestScore
  (params (HighestScore :type Integer))
  (if (> HighestScore (CallFunction|GetHighestScore))
    (Variables|Default|SetHighestScore HighestScore)))

(fn GetHighestScore
  (return (Variables|Default|GetHighestScore)))