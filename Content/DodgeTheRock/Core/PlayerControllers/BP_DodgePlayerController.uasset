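; Player controller for the DodgeTheRock game that turns Enhanced Input into movement, look, jump and pause actions for the possessed BP_DodgeCharacter.
; BeginPlay adds the mapping context and caches the character and its movement component.
; Move feeds yaw-based forward and control-rotation right vectors straight into the movement component, look adds yaw and pitch input, and jump calls the character.
; The pause action toggles game pause, a reusable pause menu widget, input mode and cursor.
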(event Input|EnhancedActionEvents|EnhancedInputActionIA_DodgeJump
  (params (ActionValue :type Boolean) (ElapsedSeconds :type Float%20%28double-precision%29) (TriggeredSeconds :type Float%20%28double-precision%29) (InputAction :type Input%20Action%20Object%20Reference :default "/Game/DodgeTheRock/Core/EnhancedInput/Action/IA_DodgeJump.IA_DodgeJump"))
  (bind _dodgecharacter (Variables|Default|GetDodgeCharacter))
  ;[0.15 0.15 0.15 0.5] Jump takes a Character; BP’s a controller, so you gotta explicitly pass DodgeCharacter — cast’s done earlier
  (:Triggered
    (Character|Jump _dodgecharacter))
  (:Completed
    (Character|StopJumping _dodgecharacter)))

(event Input|EnhancedActionEvents|EnhancedInputActionIA_DodgeTurn
  (params (ActionValue :type Vector%202D%20Structure) (ElapsedSeconds :type Float%20%28double-precision%29) (TriggeredSeconds :type Float%20%28double-precision%29) (InputAction :type Input%20Action%20Object%20Reference :default "/Game/DodgeTheRock/Core/EnhancedInput/Action/IA_DodgeTurn.IA_DodgeTurn"))
  ;[0.15 0.15 0.15 0.5] Mouse Turn
  (Class|PlayerController|AddYawInput (.x ActionValue))
  (Class|PlayerController|AddPitchInput (.y ActionValue)))

(event Input|EnhancedActionEvents|EnhancedInputActionIA_DodgePauseMenu
  (params (ActionValue :type Boolean) (ElapsedSeconds :type Float%20%28double-precision%29) (TriggeredSeconds :type Float%20%28double-precision%29) (InputAction :type Input%20Action%20Object%20Reference :default "/Game/DodgeTheRock/Core/EnhancedInput/Action/IA_DodgePauseMenu.IA_DodgePauseMenu"))
  (if (Game|IsGamePaused)
    (Game|SetGamePaused false)
    (Input|SetInputModeGameOnly self false)
    (Variables|Default|SetbShowMouseCursor false)
    (bind _pausemenuwidget (Variables|Default|GetPauseMenuWidget)
      (:then
        (Widget|RemovefromParent _pausemenuwidget))
      (:else))
    (else
      (Game|SetGamePaused true)
      (Variables|Default|GetPauseMenuWidget
        (:then
          _)
        (:else
          (bind _returnvalue (UserInterface|CreateWidget "/Game/DodgeTheRock/UI/WBP_PauseMenu.WBP_PauseMenu_C" self))
          (bind _output_get (Variables|Default|SetPauseMenuWidget _returnvalue))))
      (UserInterface|Viewport|AddtoViewport _output_get 0)
      (Input|SetInputModeGameandUI self _output_get "DoNotLock" true false)
      (Variables|Default|SetbShowMouseCursor true))))

(event Input|EnhancedActionEvents|EnhancedInputActionIA_DodgeMove
  (params (ActionValue :type Vector%202D%20Structure) (ElapsedSeconds :type Float%20%28double-precision%29) (TriggeredSeconds :type Float%20%28double-precision%29) (InputAction :type Input%20Action%20Object%20Reference :default "/Game/DodgeTheRock/Core/EnhancedInput/Action/IA_DodgeMove.IA_DodgeMove"))
  (bind _returnvalue (Pawn|GetControlRotation :!class /Script/Engine.Controller))
  ;[0.15 0.15 0.15 0.5] Move WASD
  (bind _charactermovementcomponent (Variables|Default|GetCharacterMovementComponent)
    (:then
      (Utilities|FlowControl|Sequence
        (:then_0
          ;;[0.15 0.15 0.15 0.5] Forward(Yaw)
          (Class|PawnMovementComponent|AddInputVector _charactermovementcomponent (* (.y ActionValue) (Math|Vector|GetForwardVector (Math|Rotator|MakeRotator 0.0 0.0 (.yaw (Pawn|GetControlRotation :!class /Script/Engine.Controller))))) false))
        (:then_1
          ;;[0.15 0.15 0.15 0.5] Right(roll/yaw)
          (Class|PawnMovementComponent|AddInputVector _charactermovementcomponent (* (.x ActionValue) (Math|Vector|GetRightVector (Math|Rotator|MakeRotator (.roll _returnvalue) 0.0 (.yaw _returnvalue)))) false))))
    (:else)))

(event EventBeginPlay
  (bind _self self)
  (Input|SetInputModeGameOnly _self false)
  (Variables|Default|SetbShowMouseCursor _self false)
  (Input|AddMappingContext (PlayerController|LocalPlayerSubsystems|GetEnhancedInputLocalPlayerSubsystem) "/Game/DodgeTheRock/Core/EnhancedInput/IMC_DodgeMappingContext.IMC_DodgeMappingContext" 0 "(bIgnoreAllPressedKeysUntilRelease=True,bForceImmediately=False,bNotifyUserSettings=False)")
  ;[0.15 0.15 0.15 0.5] PlayerController doesn’t own CharacterMovementComponent but has access to Pawn; if it's not a Character, Cast<ACharacter>() returns nullptr in C++ or Cast Failed in BP — recommended check the type before casting
  (bind _asbp_dodge_character (Utilities|Casting|CastToBP_DodgeCharacter (Pawn|GetControlledPawn)))
  (bind _output_get (Variables|Default|SetDodgeCharacter _asbp_dodge_character))
  (Variables|Default|SetCharacterMovementComponent (Variables|/Script/Engine.Character|GetCharacterMovement _output_get)))

(fn ConstructionScript)