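; Game state for Dodge The Rock that runs the match lifecycle, timing and scoring.
; StartGame starts a looping one-second timer that counts TimePlayed, adds RockCount to the PlayerState score and passes the time to the GameMode's Process.
; Player death ends the game, stopping the timer, sending the score to the GameInstance's SetHighestScore and calling GameMode RestartGame after a short delay.
; Its own RestartGame event reloads the current level.
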(event Custom|EndGame
  (Utilities|Time|ClearandInvalidateTimerbyHandle (Variables|Default|GetCoreGameTimer))
  (Variables|Default|SetIsGameEnded true)
  (Utilities|FlowControl|Sequence
    (:then_0
      ;[0.15 0.15 0.15 0.5] Setting HighestScore from DodgeGameInstance
      (bind _asbp_dodge_game_instance (Utilities|Casting|CastToBP_DodgeGameInstance (Game|GetGameInstance)))
      (bind _dodgeplayerstate (Variables|Default|GetDodgePlayerState)
        (:then
          (Default|SetHighestScore _asbp_dodge_game_instance (Default|GetPlayerScore _dodgeplayerstate)))
        (:else)))
    (:then_1
      (Utilities|FlowControl|Delay 2.0)
      (bind _dodgegamemode (Variables|Default|GetDodgeGameMode)
        (:then
          (Default|RestartGame _dodgegamemode))
        (:else)))))

(event Custom|RestartGame
  (bind _returnvalue (Game|GetCurrentLevelName true))
  (Game|OpenLevel(byName) (Utilities|String|StringToName _returnvalue)))

(event Custom|StartGame
  ;[0.15 0.15 0.15 0.5] Initializing CoreGameTimer, set IsGameEnded flag to false
  (bind _returnvalue (Utilities|Time|SetTimerbyEvent (EventDispatchers|CreateEvent :!event Custom|CoreGameTimeEvent) 1.0 true))
  (Variables|Default|SetCoreGameTimer _returnvalue)
  (Variables|Default|SetIsGameEnded false))

(event Custom|CoreGameTimeEvent
  ;[0.15 0.15 0.15 0.5] CoreGameTimer updates PlayerScore counter(from PlayerState); Updates TimePlayed(RockCount in the GameMode depends on)
  (bind _result (Math|Integer|IncrementInt (Variables|Default|GetTimePlayed))
    (:%20%20
      (Variables|Default|SetTimePlayed _result)
      (Utilities|FlowControl|Sequence
        (:then_0
          (bind _dodgeplayerstate (Variables|Default|GetDodgePlayerState)
            (:then
              (Default|SetPlayerScore _dodgeplayerstate (+ (Default|GetPlayerScore _dodgeplayerstate) (CallFunction|GetRockCount))))
            (:else)))
        (:then_1
          (bind _dodgegamemode (Variables|Default|GetDodgeGameMode)
            (:then
              (Default|Process _dodgegamemode (Variables|Default|GetTimePlayed)))
            (:else)))))))

(event Custom|OnPlayerDied
  (CallFunction|EndGame))

(event EventBeginPlay
  ;[0.15 0.15 0.15 0.5] Casting PlayerState and GameMode to reuse(used in CoreGameTimer in this context)
  (Utilities|FlowControl|Sequence
    (:then_0
      (bind _asbp_dodge_player_state (Utilities|Casting|CastToBP_DodgePlayerState (Game|GetPlayerState 0)))
      (Variables|Default|SetDodgePlayerState _asbp_dodge_player_state))
    (:then_1
      (bind _asbp_dodge_game_mode (Utilities|Casting|CastToBP_DodgeGameMode (Game|GetGameMode)))
      (Variables|Default|SetDodgeGameMode _asbp_dodge_game_mode))))

(fn ConstructionScript)

(fn GetRockCount
  (return (Variables|Default|GetRockCount)))

(fn SetRockCount
  (params (RockCount :type Integer))
  (Variables|Default|SetRockCount RockCount))