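; BP_DodgeCharacter is the character for DodgeTheRock, handling death as a physics ragdoll.
; When BP_HealthComponent reports the owner's death, it flags the character dead, disables input, turns off capsule collision and spring arm collision testing, and simulates physics on the mesh.
; While dead, Tick moves the actor to the mesh's world location each frame, so the actor follows the ragdoll.
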(event OnOwnerDied(BP_HealthComponent)
  (bind _mesh (Variables|Character|GetMesh))
  (Variables|Default|SetIsDead true)
  (Input|DisableInput (Game|GetPlayerController 0))
  (Variables|/Script/Engine.SpringArmComponent|SetbDoCollisionTest (Variables|Default|GetSpringArm) false)
  (Collision|SetCollisionEnabled (Variables|Collision|GetCapsuleComponent) "NoCollision")
  (Collision|SetCollisionEnabled _mesh "QueryAndPhysics")
  (Physics|SetSimulatePhysics _mesh true))

(event EventTick
  (params (DeltaSeconds :type Float%20%28single-precision%29))
  (if (Variables|Default|GetIsDead)
    (Transformation|SetActorLocation (Transformation|GetWorldLocation (Variables|Character|GetMesh)) false false)))

(fn ConstructionScript)